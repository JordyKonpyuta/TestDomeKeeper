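; BP_Ellipse moves a turret along a half-ellipse arc in the Y-Z plane around its Origin component.
; On BeginPlay it takes the arc radii from Origin's bounds and registers itself with the player's BP_ThirdPersonCharacter.
; Each tick, Speed, clamped to 0–180, acts as the angle that sets the turret's position and cosine-based roll.
; The bounds are swapped: Z extent (Height) scales Y, Y extent (Width) scales Z.
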(event EventBeginPlay
  (bind _origin (Variables|Default|GetOrigin))
  (bind _boxextent (Collision|GetComponentBounds _origin))
  (Variables|Default|SetWidth (.y _boxextent))
  (Variables|Default|SetHeight (.z _boxextent))
  (bind _asbp_third_person_character (Utilities|Casting|CastToBP_ThirdPersonCharacter (Game|GetPlayerCharacter 0)))
  (Variables|/Game/ThirdPerson/Blueprints/BP_ThirdPersonCharacter.BP_ThirdPersonCharacter_C|SetBP_Ellipse _asbp_third_person_character self))

(event EventTick
  (params (DeltaSeconds :type Float%20%28single-precision%29))
  (bind _speed (Variables|Default|GetSpeed))
  (bind _returnvalue (Math|Float|Clamp(Float) _speed 0.0 1.8e+02))
  (Transformation|SetWorldLocation (Variables|Default|GetTurret) (+ (Math|Vector|MakeVector 0.0 (* (Math|Trig|Cos(Degrees) _returnvalue) (Variables|Default|GetHeight)) (* (Math|Trig|Sin(Degrees) _returnvalue) (Variables|Default|GetWidth))) (Transformation|GetWorldLocation (Variables|Default|GetOrigin))) false false)
  (Transformation|SetWorldRotation (Variables|Default|GetTurret) (Math|Rotator|MakeRotator (* (Math|Trig|Cos(Degrees) (Math|Float|Clamp(Float) (Variables|Default|GetSpeed) 0.0 1.8e+02)) (/ (Variables|Default|GetHeight) 2.0)) 0.0 0.0) false false))

(fn ConstructionScript)