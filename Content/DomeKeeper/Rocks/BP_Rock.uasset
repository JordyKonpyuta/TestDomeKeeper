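; Breakable rock for a Dome Keeper-style game that can yield gold, water, cobalt or nothing.
; On BeginPlay it randomizes health, resource type and yield, then tints a dynamic material instance to show resistance and resource.
; Each hit on the cube removes one health, without checking what struck it.
; At zero health it adds the yield to the matching PlayerRef counter, prints the total and destroys itself.
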(event OnComponentHit(Cube)
  (params (HitComponent :type Primitive%20Component%20Object%20Reference) (OtherActor :type Actor%20Object%20Reference) (OtherComp :type Primitive%20Component%20Object%20Reference) (NormalImpulse :type Vector :default "0, 0, 0") (Hit :type Hit%20Result%20Structure%20%28by%20ref%29))
  (bind _playerref (Variables|Default|GetPlayerRef))
  (bind _playerref_2 (Variables|Default|GetPlayerRef))
  (bind _playerref_3 (Variables|Default|GetPlayerRef))
  (Math|Integer|DecrementInt (Variables|Default|GetHealth)
    (:%20%20
      (if (== (Variables|Default|GetHealth) 0)
        (switch Utilities|FlowControl|Switch|SwitchonE_RessourceType (Variables|Default|GetRessourcetype)
          (:NewEnumerator0
            (bind _output_get (Variables|/Game/ThirdPerson/Blueprints/BP_ThirdPersonCharacter.BP_ThirdPersonCharacter_C|SetGoldAmount _playerref_3 (+ (Variables|/Game/ThirdPerson/Blueprints/BP_ThirdPersonCharacter.BP_ThirdPersonCharacter_C|GetGoldAmount _playerref_3) (Variables|Default|GetRessourceGiven))))
            (Development|PrintString (Utilities|String|Append "Gold : " (Utilities|String|ToString(Integer) _output_get)) true true "(R=0.000000,G=0.660000,B=1.000000,A=1.000000)" 1e+01)
            (Actor|DestroyActor))
          (:NewEnumerator1
            (bind _output_get_2 (Variables|/Game/ThirdPerson/Blueprints/BP_ThirdPersonCharacter.BP_ThirdPersonCharacter_C|SetWaterAmount _playerref (+ (Variables|/Game/ThirdPerson/Blueprints/BP_ThirdPersonCharacter.BP_ThirdPersonCharacter_C|GetWaterAmount _playerref) (Variables|Default|GetRessourceGiven))))
            (Development|PrintString (Utilities|String|Append "Water : " (Utilities|String|ToString(Integer) _output_get_2)) true true "(R=0.000000,G=0.660000,B=1.000000,A=1.000000)" 1e+01)
            (Actor|DestroyActor))
          (:NewEnumerator2
            (bind _output_get_3 (Variables|/Game/ThirdPerson/Blueprints/BP_ThirdPersonCharacter.BP_ThirdPersonCharacter_C|SetCobaltAmount _playerref_2 (+ (Variables|/Game/ThirdPerson/Blueprints/BP_ThirdPersonCharacter.BP_ThirdPersonCharacter_C|GetCobaltAmount _playerref_2) (Variables|Default|GetRessourceGiven))))
            (Development|PrintString (Utilities|String|Append "Cobalt : " (Utilities|String|ToString(Integer) _output_get_3)) true true "(R=0.000000,G=0.660000,B=1.000000,A=1.000000)" 1e+01)
            (Actor|DestroyActor))
          (:NewEnumerator3
            (Actor|DestroyActor)))))))

(event Custom|SetMaterialColor
  (Rendering|Material|SetVectorParameterValue (Variables|Default|GetMaterial) "ResistanceColor" (Utilities|Select :Index (Variables|Default|GetHealth) :Option%200 "" :Option%201 "(R=1.000000,G=1.000000,B=1.000000,A=1.000000)" :Option%202 "(R=0.212500,G=0.212500,B=0.212500,A=1.000000)" :Option%203 "(R=0.054167,G=0.054167,B=0.054167,A=1.000000)") :!class /Script/Engine.MaterialInstanceDynamic)
  (Rendering|Material|SetVectorParameterValue (Variables|Default|GetMaterial) "RessourceColor" (Utilities|Select :Index (Variables|Default|GetRessourcetype) :NewEnumerator0 "(R=1.000000,G=0.737974,B=0.000000,A=1.000000)" :NewEnumerator1 "(R=0.000000,G=0.428203,B=1.000000,A=1.000000)" :NewEnumerator2 "(R=0.462234,G=0.000000,B=1.000000,A=1.000000)" :NewEnumerator3 "(R=0.095833,G=0.034351,B=0.000000,A=1.000000)") :!class /Script/Engine.MaterialInstanceDynamic))

(event EventBeginPlay
  (bind _returnvalue (Rendering|Material|CreateDynamicMaterialInstance (Variables|Default|GetCube) 0 "/Game/DomeKeeper/Rocks/MI_Rock.MI_Rock" "None" :!class /Script/Engine.PrimitiveComponent))
  (Variables|Default|SetMaterial _returnvalue)
  (Variables|Default|SetHealth (Math|Random|RandomIntegerinRange 1 3))
  (Variables|Default|SetRessourcetype (Utilities|Select :Index (Math|Random|RandomIntegerinRange 0 3) :Option%200 "NewEnumerator0" :Option%201 "NewEnumerator1" :Option%202 "NewEnumerator2" :Option%203 "NewEnumerator3"))
  (CallFunction|SetMaterialColor)
  (Variables|Default|SetRessourceGiven (Math|Random|RandomIntegerinRange 1 5)))

(fn ConstructionScript)