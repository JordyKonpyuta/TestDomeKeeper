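; BP_Ellipse is an actor that moves a Sphere component in the world YZ plane every Tick, apparently meant as an elliptical path around Origin.
; Each frame adds Origin's world Y plus cosine of Angle, and Z plus sine, each scaled by Radius, to the sphere's current location.
; The offset accumulates rather than setting an orbit point, and nothing shown updates Angle.
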(event EventTick
  (params (DeltaSeconds :type Float%20%28single-precision%29))
  (bind _origin (Variables|Default|GetOrigin))
  (bind _sphere (Variables|Default|GetSphere))
  (bind _returnvalue (Transformation|GetWorldLocation _sphere))
  (bind _returnvalue_2 (Transformation|GetWorldLocation _origin))
  (Transformation|SetWorldLocation _sphere (Math|Vector|MakeVector (.x _returnvalue) (+ (.y _returnvalue) (* (+ (.y _returnvalue_2) (Math|Trig|Cos(Degrees) (Variables|Default|GetAngle))) (Variables|Default|GetRadius))) (+ (.z _returnvalue) (* (+ (.z _returnvalue_2) (Math|Trig|Sin(Degrees) (Variables|Default|GetAngle))) (Variables|Default|GetRadius)))) false false))

(fn ConstructionScript)